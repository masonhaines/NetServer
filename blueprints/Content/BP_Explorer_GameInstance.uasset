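; Explorer game instance that owns the TCP client the game uses to fetch file data from a server.
; Init creates the client, a connect event registers as UnrealClient, starts async polling and re-requests data on a looping timer, and Shutdown disconnects.
; A wrapper function returns a named file's data split into lines.
; A separate event snapshots which POIs are currently showing.
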(event `ConnectAndStartPolling`
  (bind _gi_tcpclient (`self.GI_TcpClient`)
    (:`then`
      (`TcpClient.Connect` _gi_tcpclient (`self.localTestingAddress`) (`self.Server Port`))
      ;[0.02779 0.15 0.03709] connect to TCP socket and start async poll/tick
      (`TcpClient.SendMessage` _gi_tcpclient "UnrealClient" "updateName" "")
      (bind _output_get (set `self.bSocketConnected` (`TcpClient.bIsConnected` _gi_tcpclient)))
      (if _output_get
        (`TcpClient.StartPollAsynchronously` _gi_tcpclient)
        (`TcpClient.RequestData` (`self.GI_TcpClient`))
        (set `self.bCanRead` true)
        (`KismetSystemLibrary.K2_SetTimerDelegate` (delegate `requestData`) 60.0 true)))
    (:`else`)))

(event `MultiThreadedWork`)

(event `FinishedWork`)

(event `requestData`
  (`TcpClient.RequestData` (`self.GI_TcpClient`)))

(event `self.ReceiveShutdown`
  (bind _gi_tcpclient (`self.GI_TcpClient`)
    (:`then`
      (if (`TcpClient.bIsConnected` _gi_tcpclient)
        (`TcpClient.Disconnect` _gi_tcpclient)))
    (:`else`)))

(event `self.ReceiveInit`
  (bind _returnvalue (`TcpClient.CreateTcpClient` self))
  (set `self.GI_TcpClient` _returnvalue))

(event `Store_Current_Visibility`
  (`KismetArrayLibrary.Array_Clear` (`self.BP_POIs_Visible`))
  (for _array_element (`self.BP_POIs`)
    (if (`/Game/ArchVizExplorer/Blueprints/BP_POI.Showing?` _array_element)
      (`KismetArrayLibrary.Array_AddUnique` (`self.BP_POIs_Visible`) _array_element))))

(fn `GI_GetFileDataWrapper`
  (params (targetFileName :type String))
  (returns (outData :type "Array of String") (bSuccessfull :type Boolean))
  (bind _gi_tcpclient (`self.GI_TcpClient`)
    (:`then`
      (bind (_outdata _returnvalue) (`TcpClient.GetFileData` _gi_tcpclient targetFileName))
      (if _returnvalue
        (bind _output_get (set `self.TCPOutData` _outdata)))
      (return (`KismetStringLibrary.ParseIntoArray` _output_get "\\n") _returnvalue))
    (:`else`
      (`KismetSystemLibrary.PrintString` "not valid get inside of GI wrapper "))))